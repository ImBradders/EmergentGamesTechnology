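; BP_API is a trigger actor that queries a web API when the third-person character overlaps its box.
; The overlap sends an HTTP GET to the base URL plus a hardcoded person path for "Brad".
; A successful response is parsed as JSON, and each field's value is printed on screen, or an error message if parsing fails.
; Failed requests have no handling shown.
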(event OnComponentBeginOverlap(Box)
  (params (OverlappedComponent :type Primitive%20Component%20Object%20Reference) (OtherActor :type Actor%20Object%20Reference) (OtherComp :type Primitive%20Component%20Object%20Reference) (OtherBodyIndex :type Integer) (bFromSweep :type Boolean) (SweepResult :type Hit%20Result%20Structure%20%28by%20ref%29))
  (if (Class|GameplayStatics|ObjectIsA OtherActor "/Game/ThirdPerson/Blueprints/BP_ThirdPersonCharacter.BP_ThirdPersonCharacter_C")
    (bind _result_body (|HttpRequest (Utilities|String|Append (Variables|Default|GetBase%20URL) "person/" "Brad") "Get")
      (:On%20Success
        (bind (_outjsonobject _returnvalue) (Class|JsonBlueprintFunctionLibrary|FromString _result_body))
        (if _returnvalue
          (bind _fieldnames (Class|JsonBlueprintFunctionLibrary|GetFieldNames _outjsonobject))
          (for _array_element _fieldnames
            (bind (_outvalue _returnvalue_2) (|GetJsonField _outjsonobject _array_element))
            (if _returnvalue_2
              (Development|PrintString (Utilities|String|TrimTrailing _outvalue))))
          (else
            (Development|PrintString "Unable to parse to json")))))))

(event EventBeginPlay)

(event Collision|EventActorBeginOverlap
  (params (OtherActor :type Actor%20Object%20Reference)))

(event EventTick
  (params (DeltaSeconds :type Float%20%28single-precision%29)))

(fn ConstructionScript)