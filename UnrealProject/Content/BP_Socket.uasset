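; BP_Socket is a trigger actor that opens a socket connection to a local server when the third-person character overlaps its Box.
; Each received message is decoded element by element through a Map lookup, appended to the persistent Steve string and printed on screen.
; It then replies with a fixed greeting over the stored connection, while the connected and disconnected callbacks are empty.
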(event OnComponentBeginOverlap(Box)
  (params (OverlappedComponent :type Primitive%20Component%20Object%20Reference) (OtherActor :type Actor%20Object%20Reference) (OtherComp :type Primitive%20Component%20Object%20Reference) (OtherBodyIndex :type Integer) (bFromSweep :type Boolean) (SweepResult :type Hit%20Result%20Structure%20%28by%20ref%29))
  (if (Class|GameplayStatics|ObjectIsA OtherActor "/Game/ThirdPerson/Blueprints/BP_ThirdPersonCharacter.BP_ThirdPersonCharacter_C")
    (bind _connectionid (Class|TcpSocketConnection|Connect "127.0.0.1" 50001 (delegate Custom|Disconnected) (delegate Custom|Connected) (delegate Custom|Message%20Received)))))

(event Custom|Message%20Received
  (params (ConnectionId :type Integer) (Message :type Array%20of%20Bytes))
  (for _array_element Message
    (if (.ReturnValue (Utilities|Map|Find (Variables|Default|GetMap) _array_element))
      (Variables|Default|SetSteve (Utilities|String|Append (Variables|Default|GetSteve) (.Value (Utilities|Map|Find (Variables|Default|GetMap) _array_element))))))
  (Development|PrintString (Variables|Default|GetSteve))
  (Class|TcpSocketConnection|SendData (stale OnComponentBeginOverlap(Box) _connectionid) (Class|TcpSocketConnection|ToBytes(String) "hello, server!")))

(event Custom|Connected
  (params (ConnectionId :type Integer)))

(event Custom|Disconnected
  (params (ConnectionId :type Integer)))

(event EventBeginPlay)

(event Collision|EventActorBeginOverlap
  (params (OtherActor :type Actor%20Object%20Reference)))

(event EventTick
  (params (DeltaSeconds :type Float%20%28single-precision%29)))

(fn ConstructionScript)